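; Player character Blueprint for a third-person, sword-wielding character with camera-relative movement, sprinting, light and heavy attacks, and lock-on.
; Attacking and charging states gate movement, jumping and speed changes; releasing a charged heavy attack swaps the charge montage for the attack.
; Lock-on stores the closest enemy from a VisionSphere child actor while held, and BeginPlay links that sphere and the Sword child actor.
; A debug-style input reloads the current level.
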(event Custom|AttackCombo
  ;[1 1 1] Attacking
  (Class|MainCharacter|PlayAttackCombo))

(event EventBeginPlay
  ;[1 1 1] Misc.
  (bind _assword (Utilities|Casting|CastToSword (Variables|/Script/Engine.ChildActorComponent|GetChildActor (Variables|Default|GetSword))))
  (Variables|/Game/ZenosContent/Player/Sword.Sword_C|SetParent _assword self)
  (bind _asvision_sphere (Utilities|Casting|CastToVisionSphere (Variables|/Script/Engine.ChildActorComponent|GetChildActor (Variables|Default|GetVisionOrb))))
  (Variables|Default|SetTargetingOrb _asvision_sphere)
  (Variables|Default|SetCameraArm (Variables|Default|GetSpringArm)))

(event Input|ActionEvents|InputActionJump
  (params (Key :type Key%20Structure :default "None"))
  ;[1 1 1] Other Action Elements
  (:Pressed
    (if (not (or (Variables|Default|GetIsAttacking) (Variables|Default|GetIsCharging)))
      (Character|Jump)))
  (:Released
    (Character|StopJumping)))

(event Input|ActionEvents|InputActionSprint
  (params (Key :type Key%20Structure :default "None"))
  (bind _charactermovement (Variables|Character|GetCharacterMovement))
  (bind _ischarging (Variables|Default|GetIsCharging))
  ;[1 1 1] Other Action Elements
  (:Pressed
    (Variables|Default|SetIsSprinting true)
    (if (not _ischarging)
      (Variables|/Script/Engine.CharacterMovementComponent|SetMaxWalkSpeed _charactermovement 1e+03)))
  (:Released
    (Variables|Default|SetIsSprinting false)
    (if (not (or _ischarging (Variables|Default|GetIsDashing)))
      (Variables|/Script/Engine.CharacterMovementComponent|SetMaxWalkSpeed _charactermovement 5e+02))))

(event Input|ActionEvents|InputActionLight_Attack
  (params (Key :type Key%20Structure :default "None"))
  ;[1 1 1] Attacking
  (:Pressed
    (Class|MainCharacter|PlayAttackMontage false)))

(event Input|ActionEvents|InputActionReset_Stage
  (params (Key :type Key%20Structure :default "None"))
  ;[1 1 1] Misc.
  (:Released
    (bind _returnvalue (Game|GetCurrentLevelName true))
    (Game|OpenLevel(byName) (Utilities|String|StringToName _returnvalue))))

(event Input|ActionEvents|InputActionHeavy_Attack
  (params (Key :type Key%20Structure :default "None"))
  ;[1 1 1] Attacking
  (:Pressed
    (Class|MainCharacter|HeavyCharge "/Game/ZenosContent/Animation/Knight/Animations/Combat/Knight_Start_Charging.Knight_Start_Charging")
    (bind _assword (Utilities|Casting|CastToSword (Variables|/Script/Engine.ChildActorComponent|GetChildActor (Variables|Default|GetSword))))
    (Default|ResetBlade _assword))
  (:Released
    (if (Variables|Default|GetIsCharging)
      (Animation|StopAnimMontage "/Game/ZenosContent/Animation/Knight/Animations/Combat/Knight_Start_Charging.Knight_Start_Charging")
      (Class|MainCharacter|PlayAttackMontage true)
      (Variables|Default|SetIsCharging false))))

(event Input|ActionEvents|InputActionLock_On
  (params (Key :type Key%20Structure :default "None"))
  ;[1 1 1] Lock On
  (:Pressed
    (bind _returnvalue (Class|VisionOrb|FindClosestEnemy (Variables|Default|GetTargetingOrb) (Transformation|GetWorldLocation (Variables|Default|GetCapsuleComponent))))
    (Variables|Default|SetClosestTarget _returnvalue)
    (Variables|Default|SetIsLockedOn true))
  (:Released
    (Variables|Default|SetIsLockedOn false)
    (if (Utilities|IsValid (Variables|Default|GetClosestTarget))
      (Rendering|SetVisibility (Variables|/Script/Zenos.BasicEnemy|GetTargetingReticle (Variables|Default|GetClosestTarget)) false false))))

(event Input|AxisEvents|InputAxisTurn
  (params (AxisValue :type Float%20%28single-precision%29))
  ;[1 1 1] Rotation Elements
  (Class|MainCharacter|LookRight AxisValue))

(event Input|AxisEvents|InputAxisMoveForward
  (params (AxisValue :type Float%20%28single-precision%29))
  ;[1 1 1] Movement Elements
  (if (not (Variables|Default|GetIsAttacking))
    (Pawn|Input|AddMovementInput (Math|Vector|GetForwardVector (Math|Rotator|MakeRotator 0.0 0.0 (.Yaw (Math|Rotator|BreakRotator (Transformation|GetWorldRotation (Variables|Default|GetSpringArm)))))) AxisValue false)))

(event Input|AxisEvents|InputAxisMoveRight
  (params (AxisValue :type Float%20%28single-precision%29))
  ;[1 1 1] Movement Elements
  (if (not (Variables|Default|GetIsAttacking))
    (Pawn|Input|AddMovementInput (Math|Vector|GetRightVector (Math|Rotator|MakeRotator 0.0 0.0 (.Yaw (Math|Rotator|BreakRotator (Transformation|GetWorldRotation (Variables|Default|GetSpringArm)))))) AxisValue false)))

(event Input|AxisEvents|InputAxisLookUp
  (params (AxisValue :type Float%20%28single-precision%29))
  ;[1 1 1] Rotation Elements
  (Class|MainCharacter|LookUp AxisValue))

(fn ConstructionScript)